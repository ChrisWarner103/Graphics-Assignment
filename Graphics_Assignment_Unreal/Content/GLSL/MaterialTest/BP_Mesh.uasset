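; BP_Mesh is a material test actor that shows a D20 mesh with adjustable base colour, roughness and metallic values.
; On BeginPlay it randomizes the hue of the base colour and creates a dynamic material instance from M_Ground_Inst.
; Every Tick it pushes the current values into that instance, reassigns it to the mesh and prints roughness and metallic to a debug text.
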(event EventBeginPlay
  (Class|KismetMathLibrary|LinearColorSetRandomHue (Variables|Default|GetBase%20Colour))
  (bind _returnvalue (Rendering|Material|CreateDynamicMaterialInstance (Variables|Default|GetD20) 0 "/Game/StarterContent/MaterialTest/M_Ground_Inst.M_Ground_Inst" "None" :!class /Script/Engine.PrimitiveComponent))
  (Variables|Default|SetMID _returnvalue))

(event Collision|EventActorBeginOverlap
  (params (OtherActor :type Actor%20Object%20Reference)))

(event EventTick
  (params (DeltaSeconds :type Float%20%28single-precision%29))
  (Utilities|FlowControl|Sequence
    (:then_0
      ;[1 1 1] Update Material Values
      (Rendering|Material|SetVectorParameterValue (Variables|Default|GetMID) "Base Colour" (Variables|Default|GetBase%20Colour) :!class /Script/Engine.MaterialInstanceDynamic)
      (Rendering|Material|SetScalarParameterValue (Variables|Default|GetMID) "Roughness" (Variables|Default|GetRoughness) :!class /Script/Engine.MaterialInstanceDynamic)
      (Rendering|Material|SetScalarParameterValue (Variables|Default|GetMID) "Metalic" (Variables|Default|GetMetalic) :!class /Script/Engine.MaterialInstanceDynamic)
      (Rendering|Material|SetMaterial (Variables|Default|GetD20) 0 (Variables|Default|GetMID)))
    (:then_1
      (Rendering|Components|TextRender|SetText (Variables|Default|GetDebug%20Text) (Utilities|Text|ToText(String) (Utilities|String|Append "Roughness: " (Utilities|String|ToString(Float) (Variables|Default|GetRoughness)) " 
Metalic: " (Utilities|String|ToString(Float) (Variables|Default|GetMetalic))))))))

(fn ConstructionScript)