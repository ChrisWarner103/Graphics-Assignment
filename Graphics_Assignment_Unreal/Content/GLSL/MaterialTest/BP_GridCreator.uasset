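; BP_GridCreator is a material test actor that spawns a grid of BP_Mesh actors to show roughness and metallic variations.
; On BeginPlay, nested loops over RowCount and ColumnCount place each mesh at Distance intervals from the creator's location.
; Each row index sets a normalized Roughness and each column index a normalized Metalic value on the spawned mesh.
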(event EventBeginPlay
  (bind _returnvalue (Transformation|GetActorLocation))
  (bind _rowcount (Variables|Default|GetRowCount))
  (for _index (range 0 _rowcount)
    (Variables|Default|SetRoughnessValue (/ (Math|Conversions|ToFloat(Integer) _index) (Math|Conversions|ToFloat(Integer) _rowcount)))
    (for _index_2 (range 0 (Variables|Default|GetColumnCount))
      (Variables|Default|SetMetalicValue (/ (Math|Conversions|ToFloat(Integer) _index_2) (Math|Conversions|ToFloat(Integer) (Variables|Default|GetColumnCount))))
      (bind _returnvalue_2 (Game|SpawnActorfromClass "/Game/StarterContent/MaterialTest/BP_Mesh.BP_Mesh_C" (Math|Transform|MakeTransform (Math|Vector|MakeVector (+ (* _index (Variables|Default|GetDistance)) (.x _returnvalue)) (+ (* _index_2 (Variables|Default|GetDistance)) (.y _returnvalue)) (.z _returnvalue)) "0, 0, 0" "1,1,1") "Undefined" 0 0))
      (Variables|/Game/StarterContent/MaterialTest/BP_Mesh.BP_Mesh_C|SetRoughness _returnvalue_2 (Variables|Default|GetRoughnessValue))
      (Variables|/Game/StarterContent/MaterialTest/BP_Mesh.BP_Mesh_C|SetMetalic _returnvalue_2 (Variables|Default|GetMetalicValue)))))

(event Collision|EventActorBeginOverlap
  (params (OtherActor :type Actor%20Object%20Reference)))

(event EventTick
  (params (DeltaSeconds :type Float%20%28single-precision%29)))

(fn ConstructionScript)